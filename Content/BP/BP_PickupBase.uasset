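; Base pickup actor for a world item that the first-person character can pick up or swap.
; TriggerSphere overlap registers it as the character's CurrentInteractableItem and shows a prompt reading Pick Up, or Swap when the GI_MyGame inventory is full; leaving clears both.
; ItemData supplies the mesh and material, applied in the Construction Script and again through RefreshItemVisuals.
; Interact only destroys the actor; no inventory changes happen here.
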(event `self.TriggerSphere.OnComponentBeginOverlap`
  (params (OverlappedComponent :type "PrimitiveComponent Object Reference") (OtherActor :type "Actor Object Reference") (OtherComp :type "PrimitiveComponent Object Reference") (OtherBodyIndex :type Integer) (bFromSweep :type Boolean) (SweepResult :type "HitResult Structure (by ref)"))
  (bind _promptwidget (`self.PromptWidget`))
  (bind _asbp_first_person_character (cast `/Game/FirstPerson/Blueprints/BP_FirstPersonCharacter` OtherActor))
  (set `/Game/FirstPerson/Blueprints/BP_FirstPersonCharacter.CurrentInteractableItem` self _asbp_first_person_character)
  (`SceneComponent.SetVisibility` _promptwidget true false)
  (bind _asgi_my_game (cast `/Game/BP/GI_MyGame` (`GameplayStatics.GetGameInstance`)))
  (bind _aswbp_interaction_prompt (cast `/Game/BP/WBP_InteractionPrompt` (`WidgetComponent.GetUserWidgetObject` _promptwidget)))
  (if (>= (`KismetArrayLibrary.Array_Length` (`/Game/BP/GI_MyGame.Inventory` _asgi_my_game)) (`/Game/BP/GI_MyGame.MaxSlots` _asgi_my_game))
    (`/Game/BP/WBP_InteractionPrompt.SetPromptText` _aswbp_interaction_prompt "[G] Swap")
    (else
      (`/Game/BP/WBP_InteractionPrompt.SetPromptText` _aswbp_interaction_prompt "[E] Pick Up"))))

(event `self.TriggerSphere.OnComponentEndOverlap`
  (params (OverlappedComponent :type "PrimitiveComponent Object Reference") (OtherActor :type "Actor Object Reference") (OtherComp :type "PrimitiveComponent Object Reference") (OtherBodyIndex :type Integer))
  (bind _asbp_first_person_character (cast `/Game/FirstPerson/Blueprints/BP_FirstPersonCharacter` OtherActor))
  (set `/Game/FirstPerson/Blueprints/BP_FirstPersonCharacter.CurrentInteractableItem` null _asbp_first_person_character)
  (`SceneComponent.SetVisibility` (`self.PromptWidget`) false false))

(event `Interact`
  (`self.K2_DestroyActor`))

(event `RefreshItemVisuals`
  (bind _sphere (`self.Sphere`))
  (bind (_itemname _itemicon _itemtype _itemmesh _itemmaterial) (break `/Game/BP/F_ItemData` (`self.ItemData`)))
  ; Refresh Item Visuals (3D)
  (`StaticMeshComponent.SetStaticMesh` _sphere _itemmesh)
  (`PrimitiveComponent.SetMaterial` _sphere 0 _itemmaterial))

(fn `UserConstructionScript`
  (bind (_itemname _itemicon _itemtype _itemmesh _itemmaterial) (break `/Game/BP/F_ItemData` (`self.ItemData`)))
  (`StaticMeshComponent.SetStaticMesh` (`self.Sphere`) _itemmesh)
  (`PrimitiveComponent.SetMaterial` (`self.Sphere`) 0 _itemmaterial))