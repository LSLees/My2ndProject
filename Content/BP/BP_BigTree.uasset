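; BP_BigTree is a decoratable tree that shows collected stage items on forest, crystal and bakery mesh slot groups.
; BeginPlay restores saved meshes from GI_MyGame, while the trigger sphere registers the tree with the player and shows a decor prompt if inventory exists.
; PreviewTree applies the selected item's mesh to its type's slots.
; ConfirmDecorate saves that mesh, sets the next stage, clears inventory, refreshes the hotbar and notifies the player.
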(event `self.ReceiveBeginPlay`
  ; HUD
  (bind _aswbp_interaction_prompt (cast `/Game/BP/WBP_InteractionPrompt` (`WidgetComponent.GetUserWidgetObject` (`self.PromptWidget`))))
  (`/Game/BP/WBP_InteractionPrompt.SetPromptText` _aswbp_interaction_prompt "[1,2,3] Select | [F] Preview | [E] Confirm")
  (bind _asgi_my_game (cast `/Game/BP/GI_MyGame` (`GameplayStatics.GetGameInstance`)))
  (bind _savedforestmesh (`/Game/BP/GI_MyGame.SavedForestMesh` _asgi_my_game))
  (`/Engine/EditorBlueprintResources/StandardMacros.IsValid` _savedforestmesh
    (:`Is Valid`
      (for _array_element (`self.DecorSlots`)
        (`StaticMeshComponent.SetStaticMesh` _array_element _savedforestmesh)
        (`SceneComponent.SetVisibility` _array_element true false)))
    (:`Is Not Valid`
      _))
  (bind _savedcavemesh (`/Game/BP/GI_MyGame.SavedCaveMesh` _asgi_my_game))
  (`/Engine/EditorBlueprintResources/StandardMacros.IsValid` _savedcavemesh
    (:`Is Valid`
      (for _array_element_2 (`self.CrystalSlots`)
        (`StaticMeshComponent.SetStaticMesh` _array_element_2 _savedcavemesh)
        (`SceneComponent.SetVisibility` _array_element_2 true false)))
    (:`Is Not Valid`
      _))
  (bind _savedbakerymesh (`/Game/BP/GI_MyGame.SavedBakeryMesh` _asgi_my_game))
  (`/Engine/EditorBlueprintResources/StandardMacros.IsValid` _savedbakerymesh
    (:`Is Valid`
      (for _array_element_3 (`self.BakerySlots`)
        (`StaticMeshComponent.SetStaticMesh` _array_element_3 _savedbakerymesh)
        (`SceneComponent.SetVisibility` _array_element_3 true false)))))

(event `self.TriggerSphere.OnComponentBeginOverlap`
  (params (OverlappedComponent :type "PrimitiveComponent Object Reference") (OtherActor :type "Actor Object Reference") (OtherComp :type "PrimitiveComponent Object Reference") (OtherBodyIndex :type Integer) (bFromSweep :type Boolean) (SweepResult :type "HitResult Structure (by ref)"))
  (bind _asbp_first_person_character (cast `/Game/FirstPerson/Blueprints/BP_FirstPersonCharacter` OtherActor))
  (set `/Game/FirstPerson/Blueprints/BP_FirstPersonCharacter.CurrentBigTree` self _asbp_first_person_character)
  (bind _asgi_my_game (cast `/Game/BP/GI_MyGame` (`GameplayStatics.GetGameInstance`)))
  (if (> (`KismetArrayLibrary.Array_Length` (`/Game/BP/GI_MyGame.Inventory` _asgi_my_game)) 0)
    (bind _returnvalue (`|CreateWidget` "/Game/BP/WBP_TreeDecorPrompt.WBP_TreeDecorPrompt_C"))
    (bind _output_get (set `self.ActiveDecorWidget` _returnvalue))
    (`UserWidget.AddToViewport` _output_get 0)
    (`/Game/BP/WBP_NotificationToast.ShowNotification` (`/Game/FirstPerson/Blueprints/BP_FirstPersonCharacter.NotificationWidget` _asbp_first_person_character) "It's time to decorate the tree!")))

(event `self.TriggerSphere.OnComponentEndOverlap`
  (params (OverlappedComponent :type "PrimitiveComponent Object Reference") (OtherActor :type "Actor Object Reference") (OtherComp :type "PrimitiveComponent Object Reference") (OtherBodyIndex :type Integer))
  (bind _activedecorwidget (`self.ActiveDecorWidget`))
  (bind _asbp_first_person_character (cast `/Game/FirstPerson/Blueprints/BP_FirstPersonCharacter` OtherActor))
  (set `/Game/FirstPerson/Blueprints/BP_FirstPersonCharacter.CurrentBigTree` null _asbp_first_person_character)
  (`/Engine/EditorBlueprintResources/StandardMacros.IsValid` _activedecorwidget
    (:`Is Valid`
      (`Widget.RemoveFromParent` _activedecorwidget)
      (set `self.ActiveDecorWidget` null))))

(event `PreviewTree`
  ; PreviewTree
  (bind _asgi_my_game (cast `/Game/BP/GI_MyGame` (`GameplayStatics.GetGameInstance`)))
  (bind _inventory (`/Game/BP/GI_MyGame.Inventory` _asgi_my_game))
  (if (> (`KismetArrayLibrary.Array_Length` _inventory) 0)
    (bind (_output_itemname _output_itemicon _output_itemtype _output_itemmesh) (break `/Game/BP/F_ItemData` (`|GetArrayItem` _inventory (`/Game/BP/GI_MyGame.SelectedIndex` _asgi_my_game))))
    (switch `/Game/BP/E_ItemType` _output_itemtype
      (:`NewEnumerator0`
        (for _array_element (`self.DecorSlots`)
          (`StaticMeshComponent.SetStaticMesh` _array_element _output_itemmesh)
          (`SceneComponent.SetVisibility` _array_element true false)
          (set `self.IsPreviewed` true :!label _label)))
      (:`NewEnumerator1`
        (for _array_element_2 (`self.CrystalSlots`)
          (`StaticMeshComponent.SetStaticMesh` _array_element_2 _output_itemmesh)
          (`SceneComponent.SetVisibility` _array_element_2 true false)
          (goto _label)))
      (:`NewEnumerator2`
        (for _array_element_3 (`self.BakerySlots`)
          (`StaticMeshComponent.SetStaticMesh` _array_element_3 _output_itemmesh)
          (`SceneComponent.SetVisibility` _array_element_3 true false)
          (goto _label))))))

(event `ConfirmDecorate`
  ; ConfirmDecorate
  (bind _asgi_my_game (cast `/Game/BP/GI_MyGame` (`GameplayStatics.GetGameInstance`)))
  (if (`self.IsPreviewed`)
    (bind (_output_itemname _output_itemicon _output_itemtype _output_itemmesh) (break `/Game/BP/F_ItemData` (`|GetArrayItem` (`/Game/BP/GI_MyGame.Inventory` _asgi_my_game) (`/Game/BP/GI_MyGame.SelectedIndex` _asgi_my_game))))
    (switch `/Game/BP/E_ItemType` _output_itemtype
      (:`NewEnumerator0`
        (set `/Game/BP/GI_MyGame.SavedForestMesh` _output_itemmesh _asgi_my_game))
      (:`NewEnumerator1`
        (set `/Game/BP/GI_MyGame.SavedCaveMesh` _output_itemmesh _asgi_my_game))
      (:`NewEnumerator2`
        (set `/Game/BP/GI_MyGame.SavedBakeryMesh` _output_itemmesh _asgi_my_game)))
    (bind _output_get (set `self.NotificationText` (select `/Game/BP/E_ItemType` _output_itemtype :`NewEnumerator0` "Mushroom Forest complete! Ready for the Crystal Cave?" :`NewEnumerator1` "Crystal Cave complete! Ready for the Gingerbread Bakery?" :`NewEnumerator2` "Bakery complete! Ready for the Mountain?" :`NewEnumerator3` "Mountain complete! Christmas Magic restored!" :!type "Text")))
    (set `/Game/BP/GI_MyGame.CurrentStage` (select `/Game/BP/E_ItemType` _output_itemtype :`NewEnumerator0` "NewEnumerator2" :`NewEnumerator1` "NewEnumerator3" :`NewEnumerator2` "NewEnumerator4" :`NewEnumerator3` "NewEnumerator0" :!type "/Game/BP/E_LevelName Enum") _asgi_my_game)
    (`KismetArrayLibrary.Array_Clear` (`/Game/BP/GI_MyGame.Inventory` _asgi_my_game))
    (bind _asbp_first_person_character (cast `/Game/FirstPerson/Blueprints/BP_FirstPersonCharacter` (`GameplayStatics.GetPlayerCharacter` 0)))
    (`/Game/BP/WBP_Hotbar.RefreshHotbar` (`/Game/FirstPerson/Blueprints/BP_FirstPersonCharacter.HotbarWidget` _asbp_first_person_character))
    (set `self.IsPreviewed` false)
    (`/Game/BP/WBP_NotificationToast.ShowNotification` (`/Game/FirstPerson/Blueprints/BP_FirstPersonCharacter.NotificationWidget` _asbp_first_person_character) _output_get)))

(fn `UserConstructionScript`
  (set `self.DecorSlots` (`|MakeArray` (`self.DecorSlot_1`) (`self.DecorSlot_2`) (`self.DecorSlot_3`) (`self.DecorSlot_4`) (`self.DecorSlot_5`) (`self.DecorSlot_6`) (`self.DecorSlot_7`) (`self.DecorSlot_8`) (`self.DecorSlot_9`)))
  (set `self.CrystalSlots` (`|MakeArray` (`self.CrystalSlot_1`) (`self.CrystalSlot_2`) (`self.CrystalSlot_3`) (`self.CrystalSlot_4`) (`self.CrystalSlot_5`) (`self.CrystalSlot_6`) (`self.CrystalSlot_7`) (`self.CrystalSlot_8`) (`self.CrystalSlot_9`) (`self.CrystalSlot_10`)))
  (set `self.BakerySlots` (`|MakeArray` (`self.BakerySlot_1`) (`self.BakerySlot_2`) (`self.BakerySlot_3`) (`self.BakerySlot_4`) (`self.BakerySlot_5`) (`self.BakerySlot_6`) (`self.BakerySlot_7`) (`self.BakerySlot_8`) (`self.BakerySlot_9`))))